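; BP_Player is the player character Blueprint, adding a camera FOV effect for sprinting.
; It caches the camera's default FOV on BeginPlay, then a timeline lerps to the sprint FOV on sprint start and reverses on sprint stop.
; Debug prints show stamina from SGCharacterAttributes every tick and the timeline alpha during the transition.
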(event EventBeginPlay
  (Variables|Default|SetDefaultFOV (Variables|/Script/Engine.CameraComponent|GetFieldOfView (Variables|Default|GetCameraComponent))))

(event Collision|EventActorBeginOverlap
  (params (OtherActor :type Actor%20Object%20Reference)))

(event EventTick
  (params (DeltaSeconds :type Float%20%28single-precision%29))
  (Development|PrintString (Utilities|String|ToString(Float) (Class|SGCharacterAttributes|GetStamina (Variables|Default|GetSGCharacterAttributes)))))

(event EventOnStartSprint
  (bind _alpha (Timeline|SprintTimeline Play)
    (:Update
      (Development|PrintString (Utilities|String|ToString(Float) _alpha))
      (Camera|SetFieldOfView (Variables|Default|GetCameraComponent) (Math|Float|Lerp (Variables|Default|GetDefaultFOV) (Variables|Default|GetSprintFOV) _alpha)))))

(event EventOnStopSprint
  (bind _alpha (Timeline|SprintTimeline Reverse)
    (:Update
      (Development|PrintString (Utilities|String|ToString(Float) _alpha))
      (Camera|SetFieldOfView (Variables|Default|GetCameraComponent) (Math|Float|Lerp (Variables|Default|GetDefaultFOV) (Variables|Default|GetSprintFOV) _alpha)))))

(fn ConstructionScript)